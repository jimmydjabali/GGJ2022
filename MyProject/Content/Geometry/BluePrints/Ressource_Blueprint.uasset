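; Resource actor that becomes water, wood or metal through the Settype event, which swaps its mesh and scatters it randomly over the map.
; Placement re-rolls while within 1000 units of the Home_Blueprint.
; It then scans all three resource classes for neighbours within 200 units, using non-looping MultiGates to break, then re-roll once.
; The scans of the other two classes leave the distance target unconnected.
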(event Custom|Set%20type
  (params (ressource_type :type String))
  (Variables|Default|Setressource_type ressource_type)
  (if (Utilities|Enum|Equal(Enum) ressource_type "water")
    (Components|StaticMesh|SetStaticMesh (Variables|Debug|GetStaticMeshComponent) "/Game/Geometry/Model/StaticMeshes/Ressources/SM_WaterSource.SM_WaterSource")
    (Transformation|SetWorldLocation (Variables|Debug|GetStaticMeshComponent) (Math|Vector|MakeVector (Math|Random|RandomFloatinRange -4.5e+03 4e+03) (Math|Random|RandomFloatinRange -4.5e+03 4.5e+03) 2.4e+02) false true :!label _label)
    (bind _returnvalue (Actor|GetActorOfClass "/Game/Geometry/BluePrints/Home_Blueprint.Home_Blueprint_C"))
    (Math|Float|CompareFloat 1e+03 (Transformation|GetDistanceTo _returnvalue)
      (:>
        (goto _label))
      (:==
        _)
      (:<
        _))
    (bind _outactors (Actor|GetAllActorsOfClass "Ressource_Blueprint_C"))
    (bind _array_element (Utilities|Array|ForEachLoopwithBreak _outactors :!label _label_2)
      (:LoopBody
        (Math|Float|CompareFloat 2e+02 (Transformation|GetDistanceTo _array_element)
          (:>
            (Utilities|FlowControl|MultiGate false false -1
              (:Out%200
                (goto _label_2 Break))
              (:Out%201
                (goto _label))))))
      (:Completed
        (bind _outactors_2 (Actor|GetAllActorsOfClass "/Game/Geometry/BluePrints/Ressource_2_Blueprint.Ressource_2_Blueprint_C"))
        (Utilities|Array|ForEachLoopwithBreak _outactors_2 :!label _label_3
          (:LoopBody
            (Math|Float|CompareFloat 2e+02 (Transformation|GetDistanceTo 0)
              (:>
                (Utilities|FlowControl|MultiGate false false -1
                  (:Out%200
                    (goto _label_3 Break))
                  (:Out%201
                    (goto _label))))))
          (:Completed
            (bind _outactors_3 (Actor|GetAllActorsOfClass "/Game/Geometry/BluePrints/Ressource_3_Blueprint.Ressource_3_Blueprint_C"))
            (Utilities|Array|ForEachLoopwithBreak _outactors_3 :!label _label_4
              (:LoopBody
                (Math|Float|CompareFloat 2e+02 (Transformation|GetDistanceTo 0)
                  (:>
                    (Utilities|FlowControl|MultiGate false false -1
                      (:Out%200
                        (goto _label_4 Break))
                      (:Out%201
                        (goto _label)))))))))))
    (elif (Utilities|Enum|Equal(Enum) ressource_type "wood")
      (Components|StaticMesh|SetStaticMesh (Variables|Debug|GetStaticMeshComponent) "/Game/Geometry/Model/StaticMeshes/Ressources/SM_Tree.SM_Tree")
      (goto _label)
      (elif (Utilities|Enum|Equal(Enum) ressource_type "metal")
        (Components|StaticMesh|SetStaticMesh (Variables|Debug|GetStaticMeshComponent) "/Game/Geometry/Model/StaticMeshes/Ressources/SM_Metal.SM_Metal")
        (goto _label)))))

(event EventBeginPlay)

(fn ConstructionScript)