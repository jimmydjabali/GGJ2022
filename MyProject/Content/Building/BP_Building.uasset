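; BP_Building is a building actor with a configurable mesh and a red or green team color.
; The construction script applies the BuildingType mesh and creates a dynamic instance of MI_TeamColor on material slot 0, stored as MaterialInstance.
; Every Tick sets that instance's BaseColor parameter from IsTeam1, red for team 1 and green otherwise.
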(event EventBeginPlay)

(event Collision|EventActorBeginOverlap
  (params (OtherActor :type Actor%20Object%20Reference)))

(event EventTick
  (params (DeltaSeconds :type Float%20%28single-precision%29))
  (bind _materialinstance (Variables|Default|GetMaterialInstance))
  (if (Variables|Default|GetIsTeam1)
    (Rendering|Material|SetVectorParameterValue _materialinstance "BaseColor" "(R=1.000000,G=0.000000,B=0.000000,A=1.000000)" :!class /Script/Engine.MaterialInstanceDynamic)
    (else
      (Rendering|Material|SetVectorParameterValue _materialinstance "BaseColor" "(R=0.000000,G=1.000000,B=0.000000,A=1.000000)" :!class /Script/Engine.MaterialInstanceDynamic))))

(fn ConstructionScript
  (Components|StaticMesh|SetStaticMesh (Variables|Default|GetStaticMesh) (Variables|Default|GetBuildingType))
  (bind _returnvalue (Rendering|Material|CreateDynamicMaterialInstance (Variables|Default|GetStaticMesh) 0 "/Game/Geometry/Model/Material/MaterialInstances/MI_TeamColor.MI_TeamColor" "None" :!class /Script/Engine.PrimitiveComponent))
  (Variables|Default|SetMaterialInstance _returnvalue))